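; Dialogue trigger volume that passes its text and NumBool to any actor entering its box.
; Begin overlap calls FNTriggerDialoguesMessage on that actor; end overlap calls it again to clear the state, and both update the Overlapp flag.
; BeginPlay caches Bp_character, though overlaps message the other actor directly without filtering.
; SetPlace just returns the actor's location; its stage-teleport search is disconnected.
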(event OnComponentBeginOverlap(Box)
  (params (OverlappedComponent :type Primitive%20Component%20Object%20Reference) (OtherActor :type Actor%20Object%20Reference) (OtherComp :type Primitive%20Component%20Object%20Reference) (OtherBodyIndex :type Integer) (bFromSweep :type Boolean) (SweepResult :type Hit%20Result%20Structure%20%28by%20ref%29))
  (Class|BPITriggerRoof|FNTriggerDialogues(Message) OtherActor (Variables|Default|GetNum%20Bool) (Variables|Default|GetTEXT%20TO%20SHOW) true)
  (Variables|Default|SetOverlapp true))

(event OnComponentEndOverlap(Box)
  (params (OverlappedComponent :type Primitive%20Component%20Object%20Reference) (OtherActor :type Actor%20Object%20Reference) (OtherComp :type Primitive%20Component%20Object%20Reference) (OtherBodyIndex :type Integer))
  (Class|BPITriggerRoof|FNTriggerDialogues(Message) OtherActor 0 0 false)
  (Variables|Default|SetOverlapp false))

(event EventBeginPlay
  (bind _returnvalue (Actor|GetActorOfClass "/Game/Blueprints/Character/bp_character.bp_character_C"))
  (Variables|Default|SetCharacterPlayer _returnvalue))

(event EventTick
  (params (DeltaSeconds :type Float%20%28single-precision%29)))

(fn ConstructionScript)

(fn SetPlace
  (return (Transformation|GetActorLocation)))