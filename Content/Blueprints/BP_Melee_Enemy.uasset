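; BP_Melee_Enemy is a melee enemy that chases Bp_character and damages it at close range.
; EnemyStartFollow starts a looping timer that calls FNchase, which steps toward the player by local offset and sets Touching within 30 units.
; Once Touching is set, or ActionValue is false, the timer damages Objective instead; Touching then never clears, as only FNchase resets it.
; Box overlaps also send an interface damage message; HP is only initialised here.
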(event OnComponentBeginOverlap(Box)
  (params (OverlappedComponent :type Primitive%20Component%20Object%20Reference) (OtherActor :type Actor%20Object%20Reference) (OtherComp :type Primitive%20Component%20Object%20Reference) (OtherBodyIndex :type Integer) (bFromSweep :type Boolean) (SweepResult :type Hit%20Result%20Structure%20%28by%20ref%29))
  (Class|BPIDamage|BPIDamage(Message) OtherActor true (Variables|Default|GetDamage)))

(event Custom|EnemyStartFollow
  (params (Action%20Value :type Boolean))
  (Utilities|Time|SetTimerbyEvent (delegate Custom|Following) 0.3 true))

(event Custom|Following
  (if (and (not (Variables|Default|Gettouching)) (stale Custom|EnemyStartFollow Action%20Value))
    (CallFunction|FNchase)
    (else
      (Default|PlayerTakeDMG (Variables|Default|GetObjective) (Variables|Default|GetDamage)))))

(event EventBeginPlay
  (Variables|Default|SetHP%20Enemy (Variables|Default|GetHP%20Init%20Enemy)))

(fn ConstructionScript)

(fn FNchase
  (if (<= (Math|Vector|Distance(Vector) (Transformation|GetActorLocation (Variables|Default|GetObjective)) (Transformation|GetActorLocation)) 3e+01)
    (Variables|Default|Settouching true)
    (else
      (Variables|Default|Settouching false)
      (bind _returnvalue (Actor|GetActorOfClass "/Game/Blueprints/Character/bp_character.bp_character_C"))
      (Variables|Default|SetObjective _returnvalue)
      (Transformation|AddActorLocalOffset (* (Math|Vector|Normalize (- (Transformation|GetActorLocation _returnvalue) (Transformation|GetActorLocation))) (Variables|Default|GetSpeed)) false false)
      (Development|PrintText (Utilities|Text|ToText(Float) (Math|Vector|Distance(Vector) (Transformation|GetActorLocation _returnvalue) (Transformation|GetActorLocation)) "HalfToEven"))
      (if (<= (Math|Vector|Distance(Vector) (Transformation|GetActorLocation _returnvalue) (Transformation|GetActorLocation)) 3e+01)
        (Variables|Default|Settouching true)
        (else
          (Variables|Default|Settouching false))))))