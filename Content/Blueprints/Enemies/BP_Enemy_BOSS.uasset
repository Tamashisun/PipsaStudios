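; Two-phase Paper2D boss enemy that hunts the player character and opens the win condition when killed.
; Phase one uses PawnSensing to chase and deal melee damage on a cooldown, using capsule overlap and distance checks.
; AnyDamage below half health switches it to an amulet sprite, relocates it and makes it fire projectiles on sight.
; Death optionally grants a key, starts the player's timer and spawns the win trigger.
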(event OnComponentBeginOverlap(CapsuleComponent)
  (params (OverlappedComponent :type Primitive%20Component%20Object%20Reference) (OtherActor :type Actor%20Object%20Reference) (OtherComp :type Primitive%20Component%20Object%20Reference) (OtherBodyIndex :type Integer) (bFromSweep :type Boolean) (SweepResult :type Hit%20Result%20Structure%20%28by%20ref%29))
  (if (== OtherActor (Variables|Default|GetObjective))
    (Variables|Default|Settouching true)))

(event OnSeePawn(PawnSensing)
  (params (Pawn :type Pawn%20Object%20Reference))
  ;[0.1036 1 0.4193] ON SEE PAWN
  (if (not (Variables|Default|GetInstance2?))
    (Variables|Default|SetONSeePawn (== Pawn (Variables|Default|GetObjective)))
    (if (not (Variables|Default|Gettouching))
      (CallFunction|FNchase)
      (CallFunction|GetterLocation)
      (elif (Variables|Default|Gettouching)
        (if (not (Variables|Default|GetActionAtack))
          (Class|BPIDamage|BPIDamage(Message) (Variables|Default|GetObjective) true (Variables|Default|GetDamage))
          (Variables|Default|SetActionAtack true)
          (Utilities|FlowControl|Delay (Variables|Default|GetSpeedATK))
          (bind _melee_ (CallFunction|FNCheckDistance))
          (bind _output_get (Variables|Default|Settouching _melee_))
          (Development|PrintString (Utilities|String|ToString(Boolean) _output_get) true true "(R=0.000000,G=0.014750,B=1.000000,A=1.000000)")
          (Variables|Default|SetActionAtack false))
        (else
          (CallFunction|FNchase)
          (CallFunction|GetterLocation))))
    (else
      (CallFunction|SHOOTTHINGS Pawn))))

(event OnComponentEndOverlap(CapsuleComponent)
  (params (OverlappedComponent :type Primitive%20Component%20Object%20Reference) (OtherActor :type Actor%20Object%20Reference) (OtherComp :type Primitive%20Component%20Object%20Reference) (OtherBodyIndex :type Integer))
  (if (== (Variables|Default|GetObjective) OtherActor)
    (Variables|Default|Settouching false)))

(event Custom|SHOOT%20THINGS
  (params (Pawn :type Pawn%20Object%20Reference))
  ;[1 1 1] SHOOT
  (if (and (== Pawn (Variables|Default|GetObjective)) (Variables|Default|GetCanShoot?))
    (Development|PrintString "TE VEO LOQUITO " true true "(R=0.737742,G=1.000000,B=0.000000,A=1.000000)" 5.0)
    (Game|SpawnActorfromClass "/Game/Blueprints/Enemies/bp_Proyectil_Enemy.bp_Proyectil_Enemy_C" (Math|Conversions|ToTransform(Vector) (Transformation|GetWorldLocation (Variables|Default|GetProyectileShooter))) "Undefined" "MultiplyWithRoot" 0 2e+01 0.0 (Transformation|GetActorLocation (Variables|Default|GetObjective)) 1e+01 0)
    (Variables|Default|SetCanShoot? false)
    (Utilities|FlowControl|Delay 0.3)
    (Variables|Default|SetCanShoot? true)))

(event Custom|EnemyStartFollow
  (params (Action%20Value :type Boolean) (Room :type Integer) (Activate :type Array%20of%20BP%20Melee%20Enemy%20Object%20References))
  ;[1 0 0.05706] NO VA
  ;;[0.3291 1 0.7119] FN_CHECK ROOM ENEMYS
)

(event Custom|Following
  ;[1 0 0.05706] NO VA
  ;;[1 0.2636 0.03237] MOVEMENT ENEMYS
  (if (not (Variables|Default|Gettouching))
    (CallFunction|FNchase)
    (elif (Variables|Default|Gettouching)
      (Class|BPIDamage|BPIDamage(Message) (Variables|Default|GetObjective) true (Variables|Default|GetDamage))
      (Utilities|FlowControl|Delay 1.5)
      (bind _melee_ (CallFunction|FNCheckDistance))
      (bind _output_get (Variables|Default|Settouching _melee_))
      (Development|PrintString (Utilities|String|ToString(Boolean) _output_get) true true "(R=0.000000,G=0.014750,B=1.000000,A=1.000000)")
      (Variables|Default|Setchasing false)
      (else
        (CallFunction|FNchase)))))

(event Custom|FN_StartChase
  ;[1 0 0.05706] NO VA
  ;;[1 0.2636 0.03237] MOVEMENT ENEMYS
  (Utilities|Time|SetTimerbyEvent (delegate Custom|Following) 0.2 true))

(event Custom|TransformingOnPoltergeist
  (Utilities|FlowControl|Delay 1.0)
  (Rendering|Components|Sprite|SetSprite (Variables|Default|GetPaperSprite) "/Game/Art_test/Assets/ITEMS/Amuleto1_128_Sprite.Amuleto1_128_Sprite")
  (Transformation|SetActorLocation (Variables|Default|GetLocationTransformOnPoltergeist) false false))

(event EventBeginPlay
  (|CallParentFunction)
  (bind _returnvalue (Actor|GetActorOfClass "/Game/Blueprints/Character/bp_character.bp_character_C"))
  (Variables|Default|SetObjective _returnvalue))

(event EventTick
  (params (DeltaSeconds :type Float%20%28single-precision%29)))

(event Game|Damage|EventAnyDamage
  (params (Damage :type Float%20%28single-precision%29) (DamageType :type Damage%20Type%20Object%20Reference) (InstigatedBy :type Controller%20Object%20Reference) (DamageCauser :type Actor%20Object%20Reference))
  (CallFunction|FNReduceHPPC Damage)
  (Development|PrintString (Utilities|String|Append "ME QUITO " (Utilities|String|ToString(Float) Damage) "  MI VIDA ES" (Utilities|String|ToString(Float) (Variables|Default|GetPC_Health))) true true "(R=0.000000,G=0.089374,B=1.000000,A=1.000000)")
  (if (not (Variables|Default|GetInstance2?))
    (Development|PrintString "CAMBIO DE INSTANCIA ?" true true "(R=0.908962,G=0.000000,B=1.000000,A=1.000000)")
    (CallFunction|Instances (Variables|Default|GetPC_Health))))

(fn ConstructionScript)

(fn FNchase
  (bind _returnvalue (Transformation|GetActorLocation))
  (bind _set_location_objec (Variables|Default|GetSet%20Location%20Objec))
  (if (not (Variables|Default|Gettouching))
    (Rendering|Debug|DrawDebugLine _set_location_objec _returnvalue "(R=1.000000,G=0.000000,B=0.084868,A=1.000000)" 5e+01 5.0)
    (Transformation|AddActorLocalOffset (* (Math|Vector|Normalize (Variables|Default|GetSet%20Location%20Objec)) (Variables|Default|GetSpeed)) false false)
    (Transformation|SetActorRotation (Math|Rotator|FindLookatRotation _returnvalue _set_location_objec))
    (Development|PrintString (Utilities|String|ToString(Float) (Math|Vector|Distance(Vector) (Variables|Default|GetSet%20Location%20Objec) (Transformation|GetActorLocation))))
    (bind _melee_ (CallFunction|FNCheckDistance))
    (if _melee_
      (Variables|Default|Settouching true))))

(fn FNCheckDistance
  (if (Variables|Default|Gettouching)
    (if (>= (Math|Vector|Distance(Vector) (Transformation|GetActorLocation (Variables|Default|GetObjective)) (Transformation|GetActorLocation)) 6e+01)
      (return false)
      (else
        (return true)))
    (elif (<= (Math|Vector|Distance(Vector) (Transformation|GetActorLocation (Variables|Default|GetObjective)) (Transformation|GetActorLocation)) 5e+01)
      (return true)
      (else
        (return false)))))

(fn FNReduceHPPC
  (params (DMG%20recive :type Float%20%28double-precision%29))
  (bind _healt_actual (|CallParentFunction DMG%20recive))
  (if (<= _healt_actual 0.0)
    (if (Variables|Default|GetENEMY%20CLAVE)
      (Default|GetKeyDoorEnemys (Variables|Default|GetObjective)))
    (CallFunction|ActiveTimer)
    (Actor|DestroyActor)))

(fn CheckDirection
  (bind _returnvalue (Transformation|GetActorLocation))
  (bind _objective (Variables|Default|GetObjective))
  (bind _returnvalue_2 (Transformation|GetActorLocation _objective))
  (Utilities|IsValid (Variables|Default|GetPaperSprite)
    (:Is%20Valid
      (if (< (.x _returnvalue) (.x _returnvalue_2))
        (Variables|Default|SetGoingUp true)
        (else
          (Variables|Default|SetGoingUp false)))
      (if (< (.y _returnvalue) (.y _returnvalue_2))
        (Variables|Default|SetGoingRight true)
        (else
          (Variables|Default|SetGoingRight false)))
      (if (Variables|Default|GetGoingRight)
        (if (Variables|Default|GetGoingUp)
          _)
        (elif (Variables|Default|GetGoingUp)
          _)))))

(fn GetterLocation
  (Variables|Default|SetSet%20Location%20Objec (Transformation|GetActorLocation (Variables|Default|GetObjective))))

(fn Instances
  (params (HP :type Float%20%28double-precision%29))
  (if (< HP (/ (Variables|Default|GetPC_Health_MAX) 2.0))
    (Variables|Default|SetInstance2? true)
    (CallFunction|TransformingonPoltergeist)
    (else
      (Development|PrintString (Utilities|String|ToString(Float) HP)))))

(fn ActiveTimer
  (Variables|/Game/Blueprints/Character/bp_character.bp_character_C|SetTimerON (Variables|Default|GetObjective) true)
  (bind _outactors (Actor|GetAllActorsOfClass "/Game/Blueprints/Objects/BP_PointerLocation.BP_PointerLocation_C"))
  (for _array_element _outactors
    (if (== (Variables|/Game/Blueprints/Objects/BP_PointerLocation.BP_PointerLocation_C|GetName _array_element) "Win")
      (Game|SpawnActorfromClass "/Game/Blueprints/Triggers/BP_TRiggerWIN.BP_TRiggerWIN_C" (Math|Conversions|ToTransform(Vector) (Variables|/Game/Blueprints/Objects/BP_PointerLocation.BP_PointerLocation_C|GetLocationPoint _array_element)) "Undefined" "MultiplyWithRoot" 0 0))))

(fn BPIPlayerMelee
  (params (Hit :type Boolean) (DMG :type Float%20%28double-precision%29))
  (CallFunction|FNReduceHPPC DMG))

(fn FNCharm-enemy
  (params (Touched :type Boolean))
  (Variables|/Game/Blueprints/Character/bp_character.bp_character_C|SetCharmKill? (Variables|Default|GetObjective) true)
  (Development|PrintString (Utilities|String|Append "TOQUE EL AMULETO " "AHHH ME MUERO ") true true "(R=0.000000,G=0.000000,B=0.000000,A=1.000000)" 4.0)
  (Game|Damage|ApplyDamage self 25.0 0 0)
  (return true))