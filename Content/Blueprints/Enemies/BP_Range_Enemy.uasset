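; Ranged enemy that chases the player character, shoots projectiles and deals contact damage.
; Once FN_StartChase runs, a looping timer steps it toward the player; distance checks with separate enter and exit thresholds toggle touching, which sends damage through an interface.
; PawnSensing spawns a projectile aimed at the player's location on sight.
; Damage events and melee hits reduce health, destroying it at zero; charm contact flags the player and self-damages.
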(event OnComponentBeginOverlap(CapsuleComponent)
  (params (OverlappedComponent :type Primitive%20Component%20Object%20Reference) (OtherActor :type Actor%20Object%20Reference) (OtherComp :type Primitive%20Component%20Object%20Reference) (OtherBodyIndex :type Integer) (bFromSweep :type Boolean) (SweepResult :type Hit%20Result%20Structure%20%28by%20ref%29)))

(event OnSeePawn(PawnSensing)
  (params (Pawn :type Pawn%20Object%20Reference))
  (if (== Pawn (Variables|Default|GetObjective))
    (Development|PrintString "TE VEO LOQUITO " true true "(R=1.000000,G=0.154544,B=0.000000,A=1.000000)" 5.0)
    (Game|SpawnActorfromClass "/Game/Blueprints/Enemies/bp_Proyectil_Enemy.bp_Proyectil_Enemy_C" (Math|Conversions|ToTransform(Vector) (Transformation|GetWorldLocation (Variables|Default|GetboxProyectil))) "Undefined" "MultiplyWithRoot" 0 2e+01 0.0 (Transformation|GetActorLocation (Variables|Default|GetObjective)) 0)))

(event Custom|EnemyStartFollow
  (params (Action%20Value :type Boolean) (Room :type Integer) (Activate :type Array%20of%20BP%20Melee%20Enemy%20Object%20References))
  ;[0.3291 1 0.7119] FN_CHECK ROOM ENEMYS
)

(event Custom|Following
  ;[1 0.2636 0.03237] MOVEMENT ENEMYS
  (if (and (stale Custom|EnemyStartFollow Action%20Value) (not (Variables|Default|Gettouching)))
    (CallFunction|FNchase)
    (elif (Variables|Default|Gettouching)
      (Class|BPIDamage|BPIDamage(Message) (Variables|Default|GetObjective) true (Variables|Default|GetDamage))
      (Utilities|FlowControl|Delay 1.5)
      (bind _melee_ (CallFunction|FNCheckDistance))
      (bind _output_get (Variables|Default|Settouching _melee_))
      (Development|PrintString (Utilities|String|ToString(Boolean) _output_get) true true "(R=0.000000,G=0.014750,B=1.000000,A=1.000000)")
      (else
        (CallFunction|FNchase)))))

(event Custom|FN_StartChase
  ;[1 0.2636 0.03237] MOVEMENT ENEMYS
  (Utilities|Time|SetTimerbyEvent (delegate Custom|Following) 0.4 true)
  (bind _returnvalue (Actor|GetActorOfClass "/Game/Blueprints/Character/bp_character.bp_character_C"))
  (Variables|Default|SetObjective _returnvalue))

(event EventBeginPlay
  (|CallParentFunction)
  (bind _returnvalue (Actor|GetActorOfClass "/Game/Blueprints/Character/bp_character.bp_character_C"))
  (Variables|Default|SetObjective _returnvalue))

(event Game|Damage|EventAnyDamage
  (params (Damage :type Float%20%28single-precision%29) (DamageType :type Damage%20Type%20Object%20Reference) (InstigatedBy :type Controller%20Object%20Reference) (DamageCauser :type Actor%20Object%20Reference))
  (CallFunction|FNReduceHPPC Damage)
  (Development|PrintString (Utilities|String|Append "ME QUITO " (Utilities|String|ToString(Float) Damage) "  MI VIDA ES" (Utilities|String|ToString(Float) (Variables|Default|GetPC_Health))) true true "(R=0.000000,G=0.089374,B=1.000000,A=1.000000)"))

(fn ConstructionScript)

(fn FNchase
  (if (not (Variables|Default|Gettouching))
    (Transformation|AddActorLocalOffset (* (Math|Vector|Normalize (- (Transformation|GetActorLocation (Variables|Default|GetObjective)) (Transformation|GetActorLocation))) (Variables|Default|GetSpeed)) false false)
    (bind _melee_ (CallFunction|FNCheckDistance))
    (if _melee_
      (Variables|Default|Settouching true))))

(fn FNCheckDistance
  (if (Variables|Default|Gettouching)
    (if (>= (Math|Vector|Distance(Vector) (Transformation|GetActorLocation (Variables|Default|GetObjective)) (Transformation|GetActorLocation)) 72.0)
      (return false)
      (else
        (return true)))
    (elif (<= (Math|Vector|Distance(Vector) (Transformation|GetActorLocation (Variables|Default|GetObjective)) (Transformation|GetActorLocation)) 3e+01)
      (return true)
      (else
        (return false)))))

(fn FNReduceHPPC
  (params (DMG%20recive :type Float%20%28double-precision%29))
  (bind _healt_actual (|CallParentFunction DMG%20recive))
  (if (<= _healt_actual 0.0)
    (Actor|DestroyActor)))

(fn BPIPlayerMelee
  (params (Hit :type Boolean) (DMG :type Float%20%28double-precision%29))
  (CallFunction|FNReduceHPPC DMG))

(fn FNCharm-enemy
  (params (Touched :type Boolean))
  (Variables|/Game/Blueprints/Character/bp_character.bp_character_C|SetCharmKill? (Variables|Default|GetObjective) true)
  (Development|PrintString (Utilities|String|Append "TOQUE EL AMULETO " "AHHH ME MUERO ") true true "(R=0.000000,G=0.000000,B=0.000000,A=1.000000)" 4.0)
  (Game|Damage|ApplyDamage self 25.0 0 0)
  (return true))