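; Player character Blueprint with sprite-based directional movement, health, an item bag, a key-symbol bag and melee attacks.
; Enhanced Input drives movement, sprite facing, interact toggle, mouse cursor and attacks that damage overlapping enemies when the item can hit ghosts.
; Keys 1–4 select bag slots, resolving damage and ghost-hit ability from an item DataTable.
; Interface events handle damage, pickups, door prompts, roof visibility, enemy following and stage relocation.
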(event OnComponentBeginOverlap(CapsuleComponent)
  (params (OverlappedComponent :type Primitive%20Component%20Object%20Reference) (OtherActor :type Actor%20Object%20Reference) (OtherComp :type Primitive%20Component%20Object%20Reference) (OtherBodyIndex :type Integer) (bFromSweep :type Boolean) (SweepResult :type Hit%20Result%20Structure%20%28by%20ref%29))
  ;[1 1 1] Charm
  (Class|BPIGrabItems|BPIGRAB(Message) OtherActor 2)
  ;[1 1 1] Palito
  (Class|BPIGrabItems|BPIGRAB(Message) OtherActor 1))

(event OnComponentBeginOverlap(Meleeatack)
  (params (OverlappedComponent :type Primitive%20Component%20Object%20Reference) (OtherActor :type Actor%20Object%20Reference) (OtherComp :type Primitive%20Component%20Object%20Reference) (OtherBodyIndex :type Integer) (bFromSweep :type Boolean) (SweepResult :type Hit%20Result%20Structure%20%28by%20ref%29))
  (if (Variables|Booleans|GetMelee_Click)
    (Development|PrintString "Hello")
    (Class|BPIMeleeAtackPlayer|FNMELEEPLAYER(Message) OtherActor true (Variables|Default|GetDamagePJ))))

(event Custom|Breakpoint
  (bind _symbolbag (Variables|Bag&Items|GetSymbolBag))
  ;[1 0.9256 0.1935] ADd to key
  (Utilities|Array|ForEachLoopwithBreak (Variables|Bag&Items|GetSymbolBag)) ; enters at Break
)

(event Custom|AddToKeyBag
  (params (Item :type Integer) (KeyName :type Name))
  (bind _symbolbag (Variables|Bag&Items|GetSymbolBag))
  ;[1 0.9256 0.1935] ADd to key
  (Variables|Bag&Items|SetKey%20Name KeyName)
  (bind (_array_element _array_index) (Utilities|Array|ForEachLoopwithBreak (Variables|Bag&Items|GetSymbolBag))
    (:LoopBody
      (if (== _array_element "Empty")
        (Utilities|Array|SetArrayElem _symbolbag _array_index (Variables|Bag&Items|GetKey%20Name))
        (CallFunction|Breakpoint)))
    (:Completed
      (for _array_element_2 _symbolbag
        (Development|PrintString (Utilities|String|ToString(Name) _array_element_2) true true "(R=1.000000,G=0.042986,B=0.000000,A=1.000000)" 4.0)))))

(event Custom|break%20loop
  (bind _itemsbag (Variables|Bag&Items|GetItemsBag))
  ;[0.1418 0.1369 1] ADD TO BAG FN
  (Utilities|Array|ForEachLoopwithBreak (Variables|Bag&Items|GetItemsBag)) ; enters at Break
)

(event Custom|ADD%20item%20to%20bag
  (params (Item :type Integer))
  (bind _itemsbag (Variables|Bag&Items|GetItemsBag))
  ;[0.1418 0.1369 1] ADD TO BAG FN
  (Variables|Bag&Items|SetN%20Item Item)
  (bind (_array_element _array_index) (Utilities|Array|ForEachLoopwithBreak (Variables|Bag&Items|GetItemsBag))
    (:LoopBody
      (if (== _array_element 0)
        (Utilities|Array|SetArrayElem _itemsbag _array_index (Variables|Bag&Items|GetN%20Item))
        (Default|RefreshSlots (Variables|Default|GetUI%20principal) (Variables|Bag&Items|GetN%20Item))
        (CallFunction|BreakLoop)))
    (:Completed
      (for _array_element_2 _itemsbag
        (Development|PrintString (Utilities|String|ToString(Integer) _array_element_2) true true "(R=1.000000,G=0.042986,B=0.000000,A=1.000000)" 4.0)))))

(event Custom|Alt_Cursor_off
  (bind _returnvalue (Game|GetPlayerController 0))
  ;[1 1 1] ALT to show mouse
  (Variables|/Script/Engine.PlayerController|SetbShowMouseCursor _returnvalue false)
  (Variables|/Script/Engine.PlayerController|SetbEnableClickEvents _returnvalue false))

(event Input|EnhancedActionEvents|EnhancedInputActionIA_ClickAtack
  (params (ActionValue :type Boolean) (ElapsedSeconds :type Float%20%28double-precision%29) (TriggeredSeconds :type Float%20%28double-precision%29) (InputAction :type Input%20Action%20Object%20Reference :default "/Game/Blueprints/Character/IA_ClickAtack.IA_ClickAtack"))
  (bind _melee_atack (Variables|Default|GetMelee%20atack))
  ;[1 1 1] MELEE  CLICK
  (:Triggered
    (Development|SetHiddeninGame _melee_atack false true)
    (CallFunction|HitCheck))
  (:Completed
    (Development|SetHiddeninGame _melee_atack true true)))

(event Input|EnhancedActionEvents|EnhancedInputActionIA_MovementCharacterAD
  (params (ActionValue :type Float%20%28double-precision%29) (ElapsedSeconds :type Float%20%28double-precision%29) (TriggeredSeconds :type Float%20%28double-precision%29) (InputAction :type Input%20Action%20Object%20Reference :default "/Game/Blueprints/Character/IA_MovementCharacterAD.IA_MovementCharacterAD"))
  (bind _luca_sprite (Variables|Default|GetLuca_sprite))
  (bind _cube (Variables|Default|GetCube))
  ;[0.08369 1 0.2424] Movement
  (:Triggered
    (if (== ActionValue 0.0)
      (Variables|Booleans|SetLateralMove false)
      (else
        (Variables|Booleans|SetLateralMove true)
        (if (< ActionValue 0.0)
          (Variables|Booleans|SetIsMovingRight? false)
          (Transformation|SetRelativeRotation _cube "-180.000000,0.000000,0.000000" false false)
          (Rendering|Components|Sprite|SetSprite _luca_sprite "/Game/Art_test/Assets/LUCA/Side_L_Sprite.Side_L_Sprite")
          (else
            (Variables|Booleans|SetIsMovingRight? true)
            (Transformation|SetRelativeRotation _cube "0.000000,0.000000,0.000000" false false)
            (Rendering|Components|Sprite|SetSprite _luca_sprite "/Game/Art_test/Assets/LUCA/Side_R_Sprite.Side_R_Sprite")))
        (Pawn|Input|AddMovementInput "0.000000,1.000000,0.000000" ActionValue false))))
  (:Completed
    (Variables|Booleans|SetLateralMove false)))

(event Input|EnhancedActionEvents|EnhancedInputActionIA_MovementCharacterWS
  (params (ActionValue :type Float%20%28double-precision%29) (ElapsedSeconds :type Float%20%28double-precision%29) (TriggeredSeconds :type Float%20%28double-precision%29) (InputAction :type Input%20Action%20Object%20Reference :default "/Game/Blueprints/Character/IA_MovementCharacterWS.IA_MovementCharacterWS"))
  (bind _lateralmove (Variables|Booleans|GetLateralMove))
  (bind _luca_sprite (Variables|Default|GetLuca_sprite))
  (bind _cube (Variables|Default|GetCube))
  ;[0.08369 1 0.2424] Movement
  (if (not (== ActionValue 0.0))
    (if (< ActionValue 0.0)
      (Variables|Booleans|SetIsMovingup?? false)
      (if _lateralmove
        _
        (else
          (Transformation|SetRelativeRotation _cube "-90.000000,0.000000,0.000000" false false)
          (Rendering|Components|Sprite|SetSprite _luca_sprite "/Game/Art_test/Assets/LUCA/Front_Sprite.Front_Sprite")))
      (else
        (Variables|Booleans|SetIsMovingup?? true)
        (if _lateralmove
          _
          (else
            (Transformation|SetRelativeRotation _cube "90.000000,0.000000,0.000000" false false)
            (Rendering|Components|Sprite|SetSprite _luca_sprite "/Game/Art_test/Assets/LUCA/Back_Sprite.Back_Sprite")))))
    (Pawn|Input|AddMovementInput "1.000000,0.000000,0.000000" ActionValue false)))

(event Input|EnhancedActionEvents|EnhancedInputActionIA_Interact
  (params (ActionValue :type Boolean) (ElapsedSeconds :type Float%20%28double-precision%29) (TriggeredSeconds :type Float%20%28double-precision%29) (InputAction :type Input%20Action%20Object%20Reference :default "/Game/Blueprints/Character/IA_Interact.IA_Interact"))
  ;[1 1 1] E BUTTON IA
  (if (Variables|Default|GetE_button)
    (Variables|Default|SetE_button false)
    (else
      (Variables|Default|SetE_button true))))

(event Input|EnhancedActionEvents|EnhancedInputActionIA_Alt_mouse
  (params (ActionValue :type Boolean) (ElapsedSeconds :type Float%20%28double-precision%29) (TriggeredSeconds :type Float%20%28double-precision%29) (InputAction :type Input%20Action%20Object%20Reference :default "/Game/Blueprints/Character/IA_Alt_mouse.IA_Alt_mouse"))
  (bind _returnvalue (Game|GetPlayerController 0))
  ;[1 1 1] ALT to show mouse
  (:Ongoing
    (Variables|/Script/Engine.PlayerController|SetbShowMouseCursor _returnvalue true)
    (Variables|/Script/Engine.PlayerController|SetbEnableClickEvents _returnvalue true))
  (:Canceled
    (Variables|/Script/Engine.PlayerController|SetbShowMouseCursor _returnvalue false)
    (Variables|/Script/Engine.PlayerController|SetbEnableClickEvents _returnvalue false)))

(event EventBeginPlay
  (|CallParentFunction)
  (bind _asplayer_controller (Utilities|Casting|CastToPlayerController (Pawn|GetController)))
  (Input|AddMappingContext (PlayerController|LocalPlayerSubsystems|GetEnhancedInputLocalPlayerSubsystem _asplayer_controller) "/Game/Blueprints/Character/IMC_Movements.IMC_Movements" 0 "(bIgnoreAllPressedKeysUntilRelease=True,bForceImmediately=False,bNotifyUserSettings=False)")
  (CallFunction|InitialValues (Variables|Default|GetMax_health) (Utilities|Array|MakeArray 0 0 0 0) (Utilities|Array|MakeArray "Empty" "Empty" "Empty" "Empty" "Empty") 0 0 (Variables|Default|GetDamagePJ)))

(event EventTriggerRoof
  (params (Visible? :type Boolean))
  ;[1 1 1] Roof BPI
  (bind _returnvalue (Actor|GetActorOfClass "/Game/Blueprints/Objects/BP_TECHITOç.BP_TECHITOç_C"))
  (if Visible?
    (Rendering|SetVisibility (Variables|/Game/Blueprints/Objects/BP_TECHITOç.BP_TECHITOç_C|GetPlane _returnvalue) true false)
    (else
      (Rendering|SetVisibility (Variables|/Game/Blueprints/Objects/BP_TECHITOç.BP_TECHITOç_C|GetPlane _returnvalue) false false))))

(event EventFNChangeStage
  (params (NewStage :type Vector :default "0, 0, 0"))
  ;[1 1 1] TP_BPI
  (Transformation|SetActorLocation NewStage false false))

(event EventFNEnemyFollows
  (params (Follow%20value :type Boolean) (Number%20of%20room :type Integer) (List%20Of%20enemys :type Array%20of%20BP%20Melee%20Enemy%20Object%20References))
  ;[1 1 1] FOLLOWED BPI
  (bind _output_get (Variables|Booleans|SetFollowed Follow%20value))
  (bind _returnvalue (Actor|GetActorOfClass "/Game/Blueprints/Enemies/BP_Melee_Enemy.BP_Melee_Enemy_C"))
  (Default|EnemyStartFollow _returnvalue _output_get Number%20of%20room List%20Of%20enemys))

(event EventFNDoor
  (params (Overlapp :type Boolean))
  ;[1 1 1] BPI Door Show
  (Default|FNVisibleDoorLock (Variables|Default|GetUI%20principal) Overlapp)
  (if Overlapp
    _
    (else
      _))
  (Variables|Default|SetE_button false))

(event EventBPIDamage
  (params (NewParam :type Boolean) (Damage%20toPlayer :type Float%20%28double-precision%29))
  ;[1 1 1] DAMAGE BPI
  (CallFunction|PlayerTakeDMG Damage%20toPlayer))

(event EventPickObject
  (params (RangeToPick :type Boolean))
  ;[1 1 1] BPI Pick show
  (Default|FNVisiblePick (Variables|Default|GetUI%20principal) RangeToPick)
  (if RangeToPick
    _
    (else
      _))
  (Variables|Default|SetE_button false))

(event EventPickCharmAfterEvent
  (params (RangeToPick :type Boolean) (Event%20ghost :type Boolean))
  ;[1 1 1] Get Amulet after kill ghost
  (if (Variables|Booleans|GetCharmKill?)
    (Default|FNVisiblePick (Variables|Default|GetUI%20principal) RangeToPick)
    (if RangeToPick
      _
      (else
        _))
    (Variables|Default|SetE_button false)))

(event Input|KeyboardEvents|9
  (params (Key :type Key%20Structure :default "None"))
  (:Pressed
    (Transformation|SetRelativeRotation (Variables|Default|GetCube) "-90.000000,0.000000,0.000000" false false)))

(event Input|KeyboardEvents|8
  (params (Key :type Key%20Structure :default "None"))
  (:Pressed
    (CallFunction|ChangeValueBag)))

(event Input|KeyboardEvents|6
  (params (Key :type Key%20Structure :default "None"))
  (:Pressed
    (for _array_element (Variables|Bag&Items|GetItemsBag)
      (Development|PrintString (Utilities|String|ToString(Integer) _array_element) true true "(R=0.000000,G=0.046142,B=1.000000,A=1.000000)" 3.0))))

(event Input|KeyboardEvents|1
  (params (Key :type Key%20Structure :default "None"))
  ;[1 1 1] 1234
  (:Pressed
    (bind _buttonpressedn_ (Default|ShowSelected (Variables|/Game/UI/UI_OverlayPrincipal.UI_OverlayPrincipal_C|GetBPW_SelectedItem (Variables|Default|GetUI%20principal)) 1))
    (bind (_id_item _name_item _damageitem _hitghost_) (CallFunction|CheckSelectedItem _buttonpressedn_))
    (CallFunction|RefreshValuesfromInventori _damageitem _hitghost_)
    (Development|PrintString (Utilities|String|ToString(Name) _name_item))))

(event Input|KeyboardEvents|2
  (params (Key :type Key%20Structure :default "None"))
  ;[1 1 1] 1234
  (:Pressed
    (bind _buttonpressedn_ (Default|ShowSelected (Variables|/Game/UI/UI_OverlayPrincipal.UI_OverlayPrincipal_C|GetBPW_SelectedItem (Variables|Default|GetUI%20principal)) 2))
    (bind (_id_item _name_item _damageitem _hitghost_) (CallFunction|CheckSelectedItem _buttonpressedn_))
    (CallFunction|RefreshValuesfromInventori _damageitem _hitghost_)
    (Development|PrintString (Utilities|String|ToString(Name) _name_item))))

(event Input|KeyboardEvents|3
  (params (Key :type Key%20Structure :default "None"))
  ;[1 1 1] 1234
  (:Pressed
    (bind _buttonpressedn_ (Default|ShowSelected (Variables|/Game/UI/UI_OverlayPrincipal.UI_OverlayPrincipal_C|GetBPW_SelectedItem (Variables|Default|GetUI%20principal)) 3))
    (bind (_id_item _name_item _damageitem _hitghost_) (CallFunction|CheckSelectedItem _buttonpressedn_))
    (CallFunction|RefreshValuesfromInventori _damageitem _hitghost_)
    (Development|PrintString (Utilities|String|ToString(Name) _name_item))))

(event Input|KeyboardEvents|4
  (params (Key :type Key%20Structure :default "None"))
  ;[1 1 1] 1234
  (:Pressed
    (bind _buttonpressedn_ (Default|ShowSelected (Variables|/Game/UI/UI_OverlayPrincipal.UI_OverlayPrincipal_C|GetBPW_SelectedItem (Variables|Default|GetUI%20principal)) 4))
    (bind (_id_item _name_item _damageitem _hitghost_) (CallFunction|CheckSelectedItem _buttonpressedn_))
    (CallFunction|RefreshValuesfromInventori _damageitem _hitghost_)
    (Development|PrintString (Utilities|String|ToString(Name) _name_item))))

(event Input|KeyboardEvents|0
  (params (Key :type Key%20Structure :default "None"))
  (:Pressed
    (Transformation|SetRelativeRotation (Variables|Default|GetCube) "90.000000,0.000000,0.000000" false false)))

(fn ConstructionScript)

(fn InitialValues
  (params (Health :type Float%20%28double-precision%29) (Bag :type Array%20of%20Integers) (SymBag :type Array%20of%20Names) (Shield :type Integer) (Proyectile :type Integer) (Char_DMG :type Float%20%28double-precision%29))
  (Variables|Default|SetHealth_0 Health)
  (Variables|Bag&Items|SetItemsBag Bag)
  (Variables|Bag&Items|SetSymbolBag SymBag)
  (Variables|Default|Setshield Shield)
  (Variables|Default|SetDamagePJ Char_DMG))

(fn CreateUI
  (bind _asplayer_controller (Utilities|Casting|CastToPlayerController (Pawn|GetController)))
  (bind _returnvalue (UserInterface|CreateWidget "/Game/UI/UI_OverlayPrincipal.UI_OverlayPrincipal_C" _asplayer_controller))
  (bind _output_get (Variables|Default|SetUI%20principal _returnvalue))
  (UserInterface|Viewport|AddtoViewport _output_get 0))

(fn PlayerTakeDMG
  (params (dmg%20taken :type Float%20%28double-precision%29))
  (bind _output_get (Variables|Default|SetHealth_0 (- (Variables|Default|GetHealth_0) dmg%20taken)))
  (Development|PrintText (Utilities|Text|ToText(String) (Utilities|String|Append (Utilities|String|ToString(Float) _output_get) "   SALUD TOTAL "))))

(fn HitCheck
  (for _array_element (Collision|GetOverlappingActors (Variables|Default|GetMelee%20atack) "/Game/Blueprints/Enemies/BP_Melee_Enemy.BP_Melee_Enemy_C" :!class /Script/Engine.PrimitiveComponent)
    (if (Variables|Booleans|GetCanHitGhost?)
      (Game|Damage|ApplyDamage _array_element (Variables|Default|GetDamagePJ) 0 0))))

(fn FNReduceHPPC
  (params (DMG%20recive :type Float%20%28double-precision%29))
  (|CallParentFunction DMG%20recive))

(fn CheckSelectedItem
  (params (get%20slot%20selected :type Integer))
  (bind _returnvalue (- get%20slot%20selected 1))
  (bind _itemsbag (Variables|Bag&Items|GetItemsBag))
  (bind _output (Utilities|Array|Get(acopy) _itemsbag _returnvalue))
  (bind _outrownames (DataTable|GetDataTableRowNames "/Game/Blueprints/Objects/Data_item/DataTable_items.DataTable_items"))
  (for _array_element _outrownames
    (bind _returnvalue_2 (Utilities|GetDataTableRow "/Game/Blueprints/Objects/Data_item/DataTable_items.DataTable_items" _array_element)
      (:then
        (if (== _output (.ID_item (Utilities|Struct|BreakSTR_ITems _returnvalue_2)))
          (Development|PrintString (Utilities|String|ToString(Integer) _output) true true "(R=1.000000,G=0.000000,B=0.956661,A=1.000000)")
          (return (.ID_item (Utilities|Struct|BreakSTR_ITems _returnvalue_2)) (.Name (Utilities|Struct|BreakSTR_ITems _returnvalue_2)) (.Damage (Utilities|Struct|BreakSTR_ITems _returnvalue_2)) (.Can_dmg_ghost? (Utilities|Struct|BreakSTR_ITems _returnvalue_2))))))))

(fn ChangeValueBag
  (for (_array_element _array_index) (Variables|/Game/UI/UI_OverlayPrincipal.UI_OverlayPrincipal_C|GetarraySlots (Variables|Default|GetUI%20principal))
    (bind _outrownames (DataTable|GetDataTableRowNames "/Game/Blueprints/Objects/Data_item/DataTable_items.DataTable_items"))
    (for _array_element_2 _outrownames
      (bind _returnvalue (Utilities|GetDataTableRow "/Game/Blueprints/Objects/Data_item/DataTable_items.DataTable_items" _array_element_2)
        (:then
          (if (== (Class|WidgetBlueprintLibrary|GetBrushResourceasTexture2D (Variables|/Script/UMG.Image|GetBrush (Variables|/Game/UI/DragNDrop/BPW_Slot.BPW_Slot_C|GetSlotImage _array_element))) (.texture _returnvalue))
            (Utilities|Array|SetArrayElem (Variables|Bag&Items|GetItemsBag) _array_index (.id_item _returnvalue))))))))

(fn RefreshValuesfromInventori
  (params (DMG-item :type Float%20%28double-precision%29) (Avaiable%20to%20hit%20fhantom :type Boolean))
  (Variables|Default|SetDamagePJ DMG-item)
  (Variables|Booleans|SetCanHitGhost? Avaiable%20to%20hit%20fhantom))

(fn BPIPlayerMelee
  (params (Hit :type Boolean) (DMG :type Float%20%28double-precision%29))
  (return (Variables|Default|GetDamagePJ)))

(fn FNCharm-enemy
  (params (Touched :type Boolean))
  (return false))