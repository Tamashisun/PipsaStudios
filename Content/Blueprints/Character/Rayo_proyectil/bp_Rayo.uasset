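; Lightning (Rayo) projectile actor that damages what it hits, ignoring the Bp_character found at BeginPlay.
; BeginPlay rotates its Box by the signs of VectorDirection's Y and Z.
; Each Tick applies an unswept local offset from those components, remapped to negated X/Y and scaled by Speed without delta time.
; Box overlap applies damage, spawns CollisionRayo at a valid target with the same direction, then destroys the projectile.
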(event OnComponentBeginOverlap(Box)
  (params (OverlappedComponent :type Primitive%20Component%20Object%20Reference) (OtherActor :type Actor%20Object%20Reference) (OtherComp :type Primitive%20Component%20Object%20Reference) (OtherBodyIndex :type Integer) (bFromSweep :type Boolean) (SweepResult :type Hit%20Result%20Structure%20%28by%20ref%29))
  (if (!= OtherActor (Variables|Default|GetcharacterBP))
    (Game|Damage|ApplyDamage OtherActor (Variables|Default|Getdamgae) 0 0)
    (Utilities|IsValid OtherActor
      (:Is%20Valid
        (Game|SpawnActorfromClass "/Game/Blueprints/Character/Rayo_proyectil/CollisionRayo.CollisionRayo_C" (Math|Conversions|ToTransform(Vector) (Transformation|GetActorLocation OtherActor)) "Undefined" "MultiplyWithRoot" 0 (Variables|Default|GetVectorDirection) 0))
      (:Is%20Not%20Valid
        _))
    (Actor|DestroyActor)))

(event EventBeginPlay
  (bind _returnvalue (Actor|GetActorOfClass "/Game/Blueprints/Character/bp_character.bp_character_C"))
  (Variables|Default|SetcharacterBP _returnvalue)
  (CallFunction|Rotation? (Variables|Default|GetVectorDirection)))

(event Collision|EventActorBeginOverlap
  (params (OtherActor :type Actor%20Object%20Reference)))

(event EventTick
  (params (DeltaSeconds :type Float%20%28single-precision%29))
  (CallFunction|DirectionProyectile (Variables|Default|GetVectorDirection)))

(fn ConstructionScript)

(fn DirectionProyectile
  (params (Vector :type Vector))
  (Variables|Default|SetVectorDirection Vector)
  (Transformation|AddActorLocalOffset (* (* (Variables|Default|Getspeed) (Math|Vector|MakeVector (.y (Variables|Default|GetVectorDirection)) (.z (Variables|Default|GetVectorDirection)) 0.0)) "-1.000000,-1.000000,0.000000") false false))

(fn GetterActorForward)

(fn Rotation?
  (params (Direction :type Vector))
  (bind _returnvalue (> (.y Direction) 0.0))
  (if (> (.z Direction) 0.0)
    (if _returnvalue
      (Development|PrintString "SALE PARA  izquierda")
      (Transformation|AddLocalRotation (Variables|Default|GetBox) "180.000000,-90.000000,0.000000" false false)
      (else
        (Development|PrintString "SALE PARA ARRIBA ")
        (Transformation|AddLocalRotation (Variables|Default|GetBox) "180.000000,0.000000,0.000000" false false)))
    (elif _returnvalue
      (Development|PrintString "SALE PARA  abajo")
      (Transformation|AddLocalRotation (Variables|Default|GetBox) "0, 0, 0" false false)
      (else
        (Development|PrintString "SALE PARA derecha ")
        (Transformation|AddLocalRotation (Variables|Default|GetBox) "180.000000,90.000000,0.000000" false false)))))