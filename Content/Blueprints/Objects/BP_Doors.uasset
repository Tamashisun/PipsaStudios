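; Double door actor that opens when the player reaches it carrying the matching key symbol.
; On box overlap, CheckOpenDoor searches the SymbolBag of the Bp_character cached at BeginPlay for KeyToOpen; without a match, the overlapping actor gets a door message, cleared on exit.
; Opening rotates two hinges in opposite directions and swaps closed and open sprite visibility.
; MoveDoorCLOSE reverses this but is not called in this Blueprint.
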(event OnComponentBeginOverlap(Box)
  (params (OverlappedComponent :type Primitive%20Component%20Object%20Reference) (OtherActor :type Actor%20Object%20Reference) (OtherComp :type Primitive%20Component%20Object%20Reference) (OtherBodyIndex :type Integer) (bFromSweep :type Boolean) (SweepResult :type Hit%20Result%20Structure%20%28by%20ref%29))
  (bind _closed_ (CallFunction|CheckOpenDoor (Variables|Default|GetIs_Open)))
  (if _closed_
    (Class|BPIPickMe|FNDoor(Message) OtherActor true)))

(event OnComponentEndOverlap(Box)
  (params (OverlappedComponent :type Primitive%20Component%20Object%20Reference) (OtherActor :type Actor%20Object%20Reference) (OtherComp :type Primitive%20Component%20Object%20Reference) (OtherBodyIndex :type Integer))
  (Class|BPIPickMe|FNDoor(Message) OtherActor false))

(event EventBeginPlay
  (bind _returnvalue (Actor|GetActorOfClass "/Game/Blueprints/Character/bp_character.bp_character_C"))
  (Variables|Default|SetPlayer _returnvalue))

(event Collision|EventActorBeginOverlap
  (params (OtherActor :type Actor%20Object%20Reference)))

(event EventTick
  (params (DeltaSeconds :type Float%20%28single-precision%29)))

(fn ConstructionScript)

(fn CheckOpenDoor
  (params (IsOpen? :type Boolean))
  (if (not IsOpen?)
    (for _array_element (Variables|/Game/Blueprints/Character/bp_character.bp_character_C|GetSymbolBag (Variables|Default|GetPlayer))
      (if (== _array_element (Variables|Default|GetKeyToOpen))
        (bind _is_open_now (CallFunction|MoveDoorOpen))
        (Variables|Default|SetIs_Open _is_open_now)
        (return false)))
    (return true)))

(fn MoveDoorOpen
  (Transformation|AddRelativeRotation (Variables|Default|GetVisagra1) "0.000000,90.000000,0.000000" false false)
  (Transformation|AddRelativeRotation (Variables|Default|GetVisagra) "0.000000,-90.000000,0.000000" false false)
  (Rendering|SetVisibility (Variables|Default|GetPuertaAbierta) true false)
  (Rendering|SetVisibility (Variables|Default|GetPaperSprite3) false false)
  (return true))

(fn MoveDoorCLOSE
  (Transformation|AddRelativeRotation (Variables|Default|GetVisagra1) "0.000000,-90.000000,0.000000" false false)
  (Transformation|AddRelativeRotation (Variables|Default|GetVisagra) "0.000000,90.000000,0.000000" false false)
  (Rendering|SetVisibility (Variables|Default|GetPuertaAbierta) false false)
  (Rendering|SetVisibility (Variables|Default|GetPaperSprite3) true false)
  (return false))