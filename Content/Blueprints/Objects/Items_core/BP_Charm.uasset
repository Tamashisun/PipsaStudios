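; BP_Charm is a pickup actor for a charm item that the player collects into their bag.
; Box overlap sends interface messages to the overlapping actor, with an extra ghost-event pickup message for the first charm.
; BPIGRAB starts a looping timer that checks an E-button-while-overlapping state, polled on Tick.
; When that state is true, it adds the item, clears a player event flag and destroys itself.
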(event OnComponentBeginOverlap(BoxColl)
  (params (OverlappedComponent :type Primitive%20Component%20Object%20Reference) (OtherActor :type Actor%20Object%20Reference) (OtherComp :type Primitive%20Component%20Object%20Reference) (OtherBodyIndex :type Integer) (bFromSweep :type Boolean) (SweepResult :type Hit%20Result%20Structure%20%28by%20ref%29))
  (if (Variables|Default|GetFirstCharm)
    (if (not (Variables|Default|GetOverlapping))
      (Variables|Default|SetOverlapping true)
      (Class|BPIPickMe|FNCharm-enemy(Message) OtherActor true)
      (Utilities|IsValid OtherActor
        (:Is%20Valid
          (Class|BPIPickMe|PickCharmAfterEvent(Message) OtherActor true true)
          (Variables|Default|SetPressed%20E false))))
    (elif (not (Variables|Default|GetOverlapping))
      (Variables|Default|SetOverlapping true)
      (Class|BPIPickMe|PickObject(Message) OtherActor true)
      (Variables|Default|SetPressed%20E false)
      (Class|BPIPickMe|FNCharm-enemy(Message) OtherActor true))))

(event OnComponentEndOverlap(BoxColl)
  (params (OverlappedComponent :type Primitive%20Component%20Object%20Reference) (OtherActor :type Actor%20Object%20Reference) (OtherComp :type Primitive%20Component%20Object%20Reference) (OtherBodyIndex :type Integer))
  (Class|BPIPickMe|PickObject(Message) OtherActor false)
  (Variables|Default|SetOverlapping false)
  (Class|BPIPickMe|PickCharmAfterEvent(Message) OtherActor false false)
  (Class|BPIPickMe|FNCharm-enemy(Message) OtherActor false))

(event Custom|FN%20Button
  (bind _player (Variables|Default|GetPlayer))
  ;[1 1 1] Add Items to bag
  (if (stale EventTick _pressede)
    (Utilities|Time|ClearandInvalidateTimerbyHandle (stale EventBPIGRAB _returnvalue))
    (Default|ADDItemtoBag _player 2)
    (Utilities|Array|SetArrayElem (Variables|/Game/Blueprints/Character/bp_character.bp_character_C|GetArrayBooleanEvents _player) 1 false)
    (Actor|DestroyActor)))

(event EventBeginPlay
  (bind _returnvalue (Actor|GetActorOfClass "/Game/Blueprints/Character/bp_character.bp_character_C"))
  (Variables|Default|SetPlayer _returnvalue))

(event EventTick
  (params (DeltaSeconds :type Float%20%28single-precision%29))
  (bind _pressede (CallFunction|GetterEButton)))

(event EventBPIGRAB
  (params (N%20Item :type Integer))
  ;[1 1 1] Add Items to bag
  (Variables|Default|SetPressed%20E false)
  (bind _returnvalue (Utilities|Time|SetTimerbyEvent (delegate Custom|FN%20Button) 0.2 true)))

(fn ConstructionScript)

(fn GetterEButton
  (if (and (Variables|/Game/Blueprints/Character/bp_character.bp_character_C|GetE_button (Variables|Default|GetPlayer)) (Variables|Default|GetOverlapping))
    (bind _output_get (Variables|Default|SetPressed%20E true))
    (return _output_get)
    (else
      (bind _output_get_2 (Variables|Default|SetPressed%20E false))
      (return _output_get_2))))

(fn FNCharm-enemy
  (params (Touched :type Boolean)))