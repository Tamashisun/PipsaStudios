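; BP_Stick is a world pickup that the player can add to the Bp_character's bag.
; Its box overlap tracks range and sends PickObjectMessage to the overlapping actor when it enters or leaves.
; The BPIGRAB event starts a looping timer that polls the character's EButton along with the overlap flag.
; When both are true, it clears the timer, passes NItem to ADDItemToBag and destroys itself.
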(event OnComponentBeginOverlap(Box)
  (params (OverlappedComponent :type Primitive%20Component%20Object%20Reference) (OtherActor :type Actor%20Object%20Reference) (OtherComp :type Primitive%20Component%20Object%20Reference) (OtherBodyIndex :type Integer) (bFromSweep :type Boolean) (SweepResult :type Hit%20Result%20Structure%20%28by%20ref%29))
  (if (not (Variables|Default|GetOverlapping))
    (Variables|Default|SetOverlapping true)
    (Class|BPIPickMe|PickObject(Message) OtherActor true)))

(event OnComponentEndOverlap(Box)
  (params (OverlappedComponent :type Primitive%20Component%20Object%20Reference) (OtherActor :type Actor%20Object%20Reference) (OtherComp :type Primitive%20Component%20Object%20Reference) (OtherBodyIndex :type Integer))
  (Class|BPIPickMe|PickObject(Message) OtherActor false)
  (Variables|Default|SetOverlapping false))

(event Custom|FN%20Button
  ;[1 1 1] Add Items to bag
  (CallFunction|GetterEButton)
  (if (Variables|Default|GetPressed%20E)
    (Utilities|Time|ClearandInvalidateTimerbyHandle (stale EventBPIGRAB _returnvalue))
    (Default|ADDItemtoBag (Variables|Default|GetPlayer) (stale EventBPIGRAB N%20Item))
    (Actor|DestroyActor)))

(event EventBeginPlay
  (bind _returnvalue (Actor|GetActorOfClass "/Game/Blueprints/Character/bp_character.bp_character_C"))
  (Variables|Default|SetPlayer _returnvalue))

(event Collision|EventActorBeginOverlap
  (params (OtherActor :type Actor%20Object%20Reference)))

(event EventBPIGRAB
  (params (N%20Item :type Integer))
  ;[1 1 1] Add Items to bag
  (bind _returnvalue (Utilities|Time|SetTimerbyEvent (delegate Custom|FN%20Button) 0.2 true)))

(fn ConstructionScript)

(fn GetterEButton
  (bind _returnvalue (Actor|GetActorOfClass "/Game/Blueprints/Character/bp_character.bp_character_C"))
  (if (and (Variables|/Game/Blueprints/Character/bp_character.bp_character_C|GetE_button _returnvalue) (Variables|Default|GetOverlapping))
    (Variables|Default|SetPressed%20E true)
    (else
      (Variables|Default|SetPressed%20E false))))