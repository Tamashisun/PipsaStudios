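; BP_Charm is a pickup charm that the player collects into their bag with the E button.
; Box overlap sends interface messages for pickup range and charm-enemy state, with a FirstCharm variant that also flags a ghost event.
; The grab interface event starts a looping timer that polls the character's E button while overlapping, then adds the item and destroys the charm.
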(event OnComponentBeginOverlap(Box)
  (params (OverlappedComponent :type Primitive%20Component%20Object%20Reference) (OtherActor :type Actor%20Object%20Reference) (OtherComp :type Primitive%20Component%20Object%20Reference) (OtherBodyIndex :type Integer) (bFromSweep :type Boolean) (SweepResult :type Hit%20Result%20Structure%20%28by%20ref%29))
  (if (Variables|Default|GetFirstCharm)
    (if (not (Variables|Default|GetOverlapping))
      (Variables|Default|SetOverlapping true)
      (Class|BPIPickMe|FNCharm-enemy(Message) OtherActor true)
      (Utilities|IsValid OtherActor
        (:Is%20Valid
          (Class|BPIPickMe|PickCharmAfterEvent(Message) OtherActor true true)
          (Variables|Default|SetPressed%20E false))))
    (elif (not (Variables|Default|GetOverlapping))
      (Variables|Default|SetOverlapping true)
      (Class|BPIPickMe|PickObject(Message) OtherActor true)
      (Variables|Default|SetPressed%20E false)
      (Class|BPIPickMe|FNCharm-enemy(Message) OtherActor true))))

(event OnComponentEndOverlap(Box)
  (params (OverlappedComponent :type Primitive%20Component%20Object%20Reference) (OtherActor :type Actor%20Object%20Reference) (OtherComp :type Primitive%20Component%20Object%20Reference) (OtherBodyIndex :type Integer))
  (Class|BPIPickMe|PickObject(Message) OverlappedComponent false)
  (Variables|Default|SetOverlapping false)
  (Class|BPIPickMe|PickCharmAfterEvent(Message) OverlappedComponent false false)
  (Class|BPIPickMe|FNCharm-enemy(Message) OverlappedComponent false))

(event Custom|FN%20Button
  ;[1 1 1] Add Items to bag
  (CallFunction|GetterEButton)
  (if (Variables|Default|GetPressed%20E)
    (Utilities|Time|ClearandInvalidateTimerbyHandle (stale EventBPIGRAB _returnvalue))
    (Default|ADDItemtoBag (Variables|Default|GetPlayer) 1)
    (Actor|DestroyActor)))

(event EventBeginPlay
  (bind _returnvalue (Actor|GetActorOfClass "/Game/Blueprints/Character/bp_character.bp_character_C"))
  (Variables|Default|SetPlayer _returnvalue))

(event EventBPIGRAB
  (params (N%20Item :type Integer))
  ;[1 1 1] Add Items to bag
  (bind _returnvalue (Utilities|Time|SetTimerbyEvent (delegate Custom|FN%20Button) 0.4 true)))

(fn ConstructionScript)

(fn GetterEButton
  (Variables|Default|SetPressed%20E false)
  (if (and (Variables|/Game/Blueprints/Character/bp_character.bp_character_C|GetE_button (Variables|Default|GetPlayer)) (Variables|Default|GetOverlapping))
    (Variables|Default|SetPressed%20E true)
    (else
      (Variables|Default|SetPressed%20E false))))

(fn FNCharm-enemy
  (params (Touched :type Boolean)))