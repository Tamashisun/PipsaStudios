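; Sprite-based locked door that checks whether the player carries the symbol matching its KeyToOpen.
; On box overlap it searches the player's SymbolBag, swapping to the open sprite on a match or showing a door message otherwise, cleared on overlap end.
; Tick toggles the box's rigid-body hit notifications from IsOpen, which the open path sets to false.
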(event OnComponentBeginOverlap(Box)
  (params (OverlappedComponent :type Primitive%20Component%20Object%20Reference) (OtherActor :type Actor%20Object%20Reference) (OtherComp :type Primitive%20Component%20Object%20Reference) (OtherBodyIndex :type Integer) (bFromSweep :type Boolean) (SweepResult :type Hit%20Result%20Structure%20%28by%20ref%29))
  (bind _closed_ (CallFunction|CheckOpenDoor (Variables|Default|GetIs_Open)))
  (if _closed_
    (Class|BPIPickMe|FNDoor(Message) OtherActor true)))

(event OnComponentEndOverlap(Box)
  (params (OverlappedComponent :type Primitive%20Component%20Object%20Reference) (OtherActor :type Actor%20Object%20Reference) (OtherComp :type Primitive%20Component%20Object%20Reference) (OtherBodyIndex :type Integer))
  (Class|BPIPickMe|FNDoor(Message) OtherActor false))

(event EventBeginPlay
  (bind _returnvalue (Actor|GetActorOfClass "/Game/Blueprints/Character/bp_character.bp_character_C"))
  (Variables|Default|SetPlayer _returnvalue))

(event Collision|EventActorBeginOverlap
  (params (OtherActor :type Actor%20Object%20Reference)))

(event EventTick
  (params (DeltaSeconds :type Float%20%28single-precision%29))
  (CallFunction|CanGoTrough?))

(fn ConstructionScript)

(fn CheckOpenDoor
  (params (IsOpen? :type Boolean))
  (if (not IsOpen?)
    (for _array_element (Variables|/Game/Blueprints/Character/bp_character.bp_character_C|GetSymbolBag (Variables|Default|GetPlayer))
      (if (== _array_element (Variables|Default|GetKeyToOpen))
        (CallFunction|MoveDoorOpen)
        (Variables|Default|SetIs_Open false)
        (return false)))
    (return true)))

(fn MoveDoorCLOSE
  (Rendering|Components|Sprite|SetSprite (Variables|Default|GetPaperSprite) "/Game/Art_test/Assets/PuertaV_2_Sprite.PuertaV_2_Sprite")
  (return false))

(fn MoveDoorOpen
  (Rendering|Components|Sprite|SetSprite (Variables|Default|GetPaperSprite) "/Game/Art_test/Assets/T_PuertaH_1_Sprite.T_PuertaH_1_Sprite")
  (return true))

(fn CanGoTrough?
  (bind _box (Variables|Default|GetBox))
  (if (Variables|Default|GetIs_Open)
    (Class|PrimitiveComponent|SetNotifyRigidBodyCollision _box false)
    (else
      (Class|PrimitiveComponent|SetNotifyRigidBodyCollision _box true))))